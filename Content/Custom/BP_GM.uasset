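; BP_GM is a game mode Blueprint that sets up the gameplay UI, an OSC server and the player at BeginPlay.
; It adds WBP_GameplayWidget to the viewport and creates a listening OSC server, keeping references to both.
; SpawnPlayer then spawns BP_Player, and the game mode hands that player reference to the widget.
; Both the widget and the player receive a reference back to the game mode on creation.
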(event EventBeginPlay
  (bind _returnvalue (UserInterface|CreateWidget "/Game/Custom/UI/WBP_GameplayWidget.WBP_GameplayWidget_C" 0 self))
  (bind _output_get (Variables|Default|SetMenuWidgetRef _returnvalue))
  (UserInterface|Viewport|AddtoViewport _output_get 0)
  (bind _returnvalue_2 (Class|OSCManager|CreateOSCServer "" 9002 false true "CubeServ" 0))
  (Variables|Default|SetOscServerRef _returnvalue_2)
  (CallFunction|SpawnPlayer)
  (Variables|/Game/Custom/UI/WBP_GameplayWidget.WBP_GameplayWidget_C|SetPlayerRef (Variables|Default|GetMenuWidgetRef) (Variables|Default|GetPlayerRef)))

(fn ConstructionScript)

(fn SpawnPlayer
  (bind _returnvalue (Game|SpawnActorfromClass "/Game/Custom/Player/BP_Player.BP_Player_C" (Math|Transform|MakeTransform "0, 0, 0" "0, 0, 0" "1.000000,1.000000,1.000000") "Undefined" "MultiplyWithRoot" 0 self 0))
  (Variables|Default|SetPlayerRef _returnvalue))