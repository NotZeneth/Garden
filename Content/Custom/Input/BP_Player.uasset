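; Player actor steered by a phone's rotation sensor, received through an OSC server it creates on BeginPlay.
; Rotation-vector messages become a quaternion, offset by the calibrated inverse, that drives a spawned BP_Gyro proxy.
; Each tick, proxy roll beyond a dead zone orbits the player around the world origin, while pitch tilts its origin-facing rotation.
; Calibrate stores the current phone orientation as neutral and resets both rotations.
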(event Custom|OnMessageReceived
  (params (Message :type OSC%20Message%20Structure%20%28by%20ref%29) (IPAddress :type String) (Port :type Integer))
  (bind _output_get (Variables|Default|SetCurrentMessage Message))
  (bind _returnvalue (Class|OSCManager|GetOSCMessageAddress _output_get))
  (bind _returnvalue_2 (Class|OSCManager|GetOSCAddressFullPath _returnvalue))
  (switch string _returnvalue_2
    (:/rotationvector
      (CallFunction|RotateMesh))))

(event EventBeginPlay
  (bind _returnvalue (Class|OSCManager|CreateOSCServer "" 9002 false true "CubeServ" 0))
  (bind _output_get (Variables|Default|SetOscServer _returnvalue))
  (EventDispatchers|BindEventtoOnOscMessageReceived _output_get (delegate Custom|OnMessageReceived))
  (Transformation|SetActorLocation "1000.000000,0.000000,0.000000" false false)
  (bind _returnvalue_2 (Game|SpawnActorfromClass "/Game/Custom/Input/BP_Gyro.BP_Gyro_C" (Math|Transform|MakeTransform "0, 0, 0" "0, 0, 0" "1.000000,1.000000,1.000000") "AlwaysSpawn" "MultiplyWithRoot" 0 0))
  (Variables|Default|SetGyroRef _returnvalue_2))

(event EventTick
  (params (DeltaSeconds :type Float%20%28single-precision%29))
  (CallFunction|MoveMesh DeltaSeconds))

(fn ConstructionScript)

(fn GetMouvOffset
  (Utilities|FlowControl|Sequence
    (:then_0
      (bind _value (Class|OSCManager|GetFloat (Variables|Default|GetCurrentMessage))))
    (:then_1
      (bind _value_2 (Class|OSCManager|GetFloat (Variables|Default|GetCurrentMessage) 1)))
    (:then_2
      (bind _value_3 (Class|OSCManager|GetFloat (Variables|Default|GetCurrentMessage) 2))
      (Variables|Default|SetMessageOffset (Math|Vector|MakeVector _value _value_2 _value_3)))))

(fn RotateMesh
  ;[0.15 0.15 0.15 0.5] Gets the rotation of the phone
  (Utilities|FlowControl|Sequence
    (:then_0
      (bind _value (Class|OSCManager|GetFloat (Variables|Default|GetCurrentMessage))))
    (:then_1
      (bind _value_2 (Class|OSCManager|GetFloat (Variables|Default|GetCurrentMessage) 1)))
    (:then_2
      (bind _value_3 (Class|OSCManager|GetFloat (Variables|Default|GetCurrentMessage) 2)))
    (:then_3
      (bind _value_4 (Class|OSCManager|GetFloat (Variables|Default|GetCurrentMessage) 3))
      (bind _output_get (Variables|Default|SetPhoneRotation (Class|KismetMathLibrary|QuatNormalized (Class|KismetMathLibrary|MakeQuat _value _value_2 _value_3 _value_4) 0.0001)))
      (bind _output_get_2 (Variables|Default|SetCubeDesiredRotation (* (Class|KismetMathLibrary|QuatInversed (Variables|Default|GetInitialRotation)) _output_get)))
      (Class|MyBlueprintFunctionLibrary|SetActorWorldRotationQuat (Variables|Default|GetGyroRef) _output_get_2 false false false))))

(fn MoveMesh
  (params (DeltaTime :type Float%20%28double-precision%29))
  (bind _returnvalue (Transformation|GetActorLocation))
  (bind _gyroref (Variables|Default|GetGyroRef))
  (bind _returnvalue_2 (Transformation|GetActorRotation _gyroref))
  (bind _returnvalue_3 (Math|Rotator|FindLookatRotation _returnvalue (Math|Vector|MakeVector 0.0 0.0 0.0)))
  (Utilities|FlowControl|Sequence
    (:then_0
      (if (or (> (.roll _returnvalue_2) 1e+01) (< (.roll _returnvalue_2) -1e+01))
        (Variables|Default|SetAngle (+ (Variables|Default|GetAngle) (* (.roll _returnvalue_2) (Variables|Default|GetSpeed) DeltaTime)))
        (Transformation|SetActorLocation (Math|Vector|MakeVector (* (Math|Trig|Cos(Radians) (+ (Variables|Default|GetAngle) (* (.roll _returnvalue_2) (Variables|Default|GetSpeed) DeltaTime))) (Variables|Default|GetRadius)) (* (Math|Trig|Sin(Radians) (+ (Variables|Default|GetAngle) (* (.roll _returnvalue_2) (Variables|Default|GetSpeed) DeltaTime))) (Variables|Default|GetRadius)) 3e+02) false false)))
    (:then_1
      (Transformation|SetActorRotation (Math|Rotator|MakeRotator (.roll _returnvalue_3) (+ (.pitch _returnvalue_3) (.pitch _returnvalue_2)) (.yaw _returnvalue_3))))))

(fn Calibrate
  (bind _returnvalue (Transformation|GetActorLocation))
  (bind _returnvalue_2 (Math|Rotator|FindLookatRotation _returnvalue (Math|Vector|MakeVector 0.0 0.0 0.0)))
  (Transformation|SetActorRotation (Variables|Default|GetGyroRef))
  (Variables|Default|SetInitialRotation (Variables|Default|GetPhoneRotation))
  (Transformation|SetActorRotation (Math|Rotator|MakeRotator (.roll _returnvalue_2) (.pitch _returnvalue_2) (.yaw _returnvalue_2))))