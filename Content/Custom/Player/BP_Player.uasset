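; Player pawn steered by a phone's rotation, received over OSC, to circle the world origin and place meshes through a spawned BP_Pointer.
; Rotation quaternions drive two proxy gyro actors, one calibrated shortly after BeginPlay and one raw.
; The raw gyro's arrow tilts set orbit speed and pick one of four faces, shown as menu seasons.
; Calibrated pitch, corrected per face, aims the pawn; mouse buttons spawn meshes, randomize their set or reset after game over.
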(event Custom|StartGame
  (bind _returnvalue (Game|SpawnActorfromClass "/Game/Custom/Blueprint/BP_Pointer.BP_Pointer_C" (Math|Transform|MakeTransform "0.000000,0.000000,45000.000000" "0, 0, 0" "1.000000,1.000000,1.000000") "Undefined" "MultiplyWithRoot" 0 0))
  (Variables|Default|SetPointerRef _returnvalue)
  (Variables|Default|SetisPlaying true))

(event Custom|OnMessageReceived
  (params (Message :type OSC%20Message%20Structure%20%28by%20ref%29) (IPAddress :type String) (Port :type Integer))
  ;[0 0 1 0.5] Comment
  (bind _output_get (Variables|Misc|SetCurrentMessage Message))
  (bind _returnvalue (Class|OSCManager|GetOSCMessageAddress _output_get))
  (bind _returnvalue_2 (Class|OSCManager|GetOSCAddressFullPath _returnvalue))
  (switch string _returnvalue_2
    (:/rotationvector
      (CallFunction|RotateGyro))))

(event Custom|SpawnItem
  ;[0.15 0.15 0.15 0.5] Comment
  (if (and (Variables|Default|GetGameOver) (Variables|Default|GetisPlaying))
    (Default|ResetGame (Variables|Default|GetGameModeRef))
    (Variables|Default|SetisPlaying false)
    (else
      (Class|RadiusSpawner|SpawnMeshesinRadius (Variables|Default|GetPointerRef) false)
      (Development|PrintString "Hello"))))

(event EventBeginPlay
  ;[0 0 1 0.5] Comment
  (bind _output_get (Variables|Misc|SetOscServer (Variables|/Game/Custom/BP_GM.BP_GM_C|GetOscServerRef (Variables|Default|GetGameModeRef))))
  (EventDispatchers|BindEventtoOnOscMessageReceived _output_get (delegate Custom|OnMessageReceived))
  (CallFunction|SetPlayerBaseLocation)
  (CallFunction|SpawnGyros)
  (Utilities|FlowControl|Delay 1.0)
  (CallFunction|Calibrate))

(event EventTick
  (params (DeltaSeconds :type Float%20%28single-precision%29))
  ;[0 1 0] Comment
  (CallFunction|MoveMesh DeltaSeconds))

(event EventPossessed
  (params (NewController :type Controller%20Object%20Reference))
  ;[0.15 0.15 0.15 0.5] Comment
  (bind _asbp_player_controller (Utilities|Casting|CastToBP_PlayerController NewController))
  (bind _output_get (Variables|/Game/Custom/BP_GM.BP_GM_C|SetControllerRef (Variables|Default|GetGameModeRef) _asbp_player_controller))
  (Default|ShowMouse _output_get true))

(event Input|MouseEvents|LeftMouseButton
  (params (Key :type Key%20Structure :default "None"))
  (:Pressed
    (CallFunction|SpawnItem)))

(event Input|MouseEvents|RightMouseButton
  (params (Key :type Key%20Structure :default "None"))
  (:Pressed
    (Class|RadiusSpawner|SetMeshSetIndex (Variables|Default|GetPointerRef) (Math|Random|RandomIntegerinRange 0 2))))

(fn ConstructionScript)

(fn RotateGyro
  ;[0 0 0 0.5] Gets the rotation of the phone
  (Utilities|FlowControl|Sequence
    (:then_0
      (bind _value (Class|OSCManager|GetFloat (Variables|Misc|GetCurrentMessage))))
    (:then_1
      (bind _value_2 (Class|OSCManager|GetFloat (Variables|Misc|GetCurrentMessage) 1)))
    (:then_2
      (bind _value_3 (Class|OSCManager|GetFloat (Variables|Misc|GetCurrentMessage) 2)))
    (:then_3
      (bind _value_4 (Class|OSCManager|GetFloat (Variables|Misc|GetCurrentMessage) 3))
      (bind _output_get (Variables|Rotation|SetPhoneRotation (Class|KismetMathLibrary|QuatNormalized (Class|KismetMathLibrary|MakeQuat _value _value_2 _value_3 _value_4) 0.0001)))
      (bind _output_get_2 (Variables|Rotation|SetCubeDesiredRotation (* (Class|KismetMathLibrary|QuatInversed (Variables|Rotation|GetInitialRotation)) _output_get)))
      (Class|MyBlueprintFunctionLibrary|SetActorWorldRotationQuat (Variables|Misc|GetGyroRef) _output_get_2 false false false)
      (CallFunction|GetCurrentFace)
      (Class|MyBlueprintFunctionLibrary|SetActorWorldRotationQuat (Variables|Misc|GetPhoneGyroRef) (Variables|Rotation|GetPhoneRotation) false false false))))

(fn MoveMesh
  (params (DeltaTime :type Float%20%28double-precision%29))
  (bind _phonegyroref (Variables|Misc|GetPhoneGyroRef))
  (bind _greenarrow (Variables|/Game/Custom/Player/BP_GyroPhone.BP_GyroPhone_C|GetGreenArrow _phonegyroref))
  (bind _dot (CallFunction|GetRotationDot _greenarrow))
  (if (Variables|Default|GetisPlaying)
    (Utilities|FlowControl|Sequence
      (:then_0
        (if (or (> _dot 0.15) (< _dot -0.15))
          (bind (_x _y) (CallFunction|GetNewPosition DeltaTime))
          (Transformation|SetActorLocation (Math|Vector|MakeVector _x _y (- (Variables|Config|GetRadius) (Variables|Config|GetRadiusOffset))) false false)))
      (:then_1
        (CallFunction|RotateLaser)))))

(fn Calibrate
  (bind _returnvalue (Transformation|GetActorLocation))
  (bind _returnvalue_2 (Math|Rotator|FindLookatRotation _returnvalue (Math|Vector|MakeVector 0.0 0.0 0.0)))
  (Transformation|SetActorRotation (Variables|Misc|GetGyroRef))
  (Variables|Rotation|SetInitialRotation (Variables|Rotation|GetPhoneRotation))
  (Transformation|SetActorRotation (Math|Rotator|MakeRotator (.roll _returnvalue_2) (.pitch _returnvalue_2) (.yaw _returnvalue_2)))
  (Variables|Default|SetCurrentFace 0))

(fn GetNewPosition
  (params (DeltaTime :type Float%20%28double-precision%29))
  (Variables|Rotation|SetAngle (+ (Variables|Rotation|GetAngle) (* DeltaTime (Variables|Config|GetSpeed) (* (CallFunction|GetRotationDot (Variables|/Game/Custom/Player/BP_GyroPhone.BP_GyroPhone_C|GetGreenArrow (Variables|Misc|GetPhoneGyroRef))) -1.0))))
  (return (* (Variables|Config|GetRadius) (Math|Trig|Cos(Radians) (+ (Variables|Rotation|GetAngle) (* DeltaTime (Variables|Config|GetSpeed) (* (CallFunction|GetRotationDot (Variables|/Game/Custom/Player/BP_GyroPhone.BP_GyroPhone_C|GetGreenArrow (Variables|Misc|GetPhoneGyroRef))) -1.0))))) (* (Math|Trig|Sin(Radians) (+ (Variables|Rotation|GetAngle) (* DeltaTime (Variables|Config|GetSpeed) (* (CallFunction|GetRotationDot (Variables|/Game/Custom/Player/BP_GyroPhone.BP_GyroPhone_C|GetGreenArrow (Variables|Misc|GetPhoneGyroRef))) -1.0)))) (Variables|Config|GetRadius))))

(fn GetCurrentFace
  (bind _phonegyroref (Variables|Misc|GetPhoneGyroRef))
  (bind _bluearrow (Variables|/Game/Custom/Player/BP_GyroPhone.BP_GyroPhone_C|GetBlueArrow _phonegyroref))
  (bind _redarrow (Variables|/Game/Custom/Player/BP_GyroPhone.BP_GyroPhone_C|GetRedArrow _phonegyroref))
  (bind _dot (CallFunction|GetRotationDot _bluearrow))
  (bind _dot_2 (CallFunction|GetRotationDot _redarrow))
  (bind _returnvalue (Class|KismetMathLibrary|DegAtan2 _dot _dot_2))
  (Variables|Default|SetCurrentAngle (Math|Float|%(Float) (+ _returnvalue 1.8e+02) 3.6e+02))
  (if (and (> _returnvalue 45.0) (<= _returnvalue 135.0))
    (CallFunction|CheckDifferenteFace)
    (Default|UpdateSeason (Variables|/Game/Custom/BP_GM.BP_GM_C|GetMenuWidgetRef (Variables|Default|GetGameModeRef)))
    (elif (and (> _returnvalue -135.0) (<= _returnvalue -45.0))
      (CallFunction|CheckDifferenteFace 2)
      (Default|UpdateSeason (Variables|/Game/Custom/BP_GM.BP_GM_C|GetMenuWidgetRef (Variables|Default|GetGameModeRef)) 2)
      (elif (and (> _returnvalue -45.0) (<= _returnvalue 45.0))
        (CallFunction|CheckDifferenteFace 1)
        (Default|UpdateSeason (Variables|/Game/Custom/BP_GM.BP_GM_C|GetMenuWidgetRef (Variables|Default|GetGameModeRef)) 1)
        (elif (or (> _returnvalue 135.0) (<= _returnvalue -135.0))
          (CallFunction|CheckDifferenteFace 3)
          (Default|UpdateSeason (Variables|/Game/Custom/BP_GM.BP_GM_C|GetMenuWidgetRef (Variables|Default|GetGameModeRef)) 3))))))

(fn RotateLaser
  (bind _returnvalue (Transformation|GetActorLocation))
  (bind _returnvalue_2 (Math|Vector|MakeVector 0.0 0.0 0.0))
  (bind _returnvalue_3 (Math|Rotator|FindLookatRotation _returnvalue _returnvalue_2))
  ;[0.15 0.15 0.15 0.5] Comment
  (Transformation|SetActorRotation (Math|Rotator|MakeRotator (.roll _returnvalue_3) (Math|Float|Clamp(Float) (+ (.pitch _returnvalue_3) (* (.pitch (Class|KismetMathLibrary|QuatRotator (* (Class|MyBlueprintFunctionLibrary|GetActorWorldRotationQuat (Variables|Misc|GetGyroRef)) (Math|Conversions|ToQuaternion(Rotator) (Utilities|Select :Index (Variables|Default|GetCurrentFace) :Option%200 "0, 0, 0" :Option%201 "90.000000,0.000000,0.000000" :Option%202 "180.000000,0.000000,0.000000" :Option%203 "-90.000000,0.000000,0.000000"))))) (Math|Float|SelectFloat 1.0 -1.0 (or (== (Variables|Default|GetCurrentFace) 0) (== (Variables|Default|GetCurrentFace) 2))) 1.0)) -7e+01 -25.0) (.yaw _returnvalue_3))))

(fn CheckDifferenteFace
  (params (NewFace :type Integer))
  (if (!= NewFace (Variables|Default|GetCurrentFace))
    (Development|PrintString (Utilities|String|Append "New face : " "from " (Utilities|String|ToString(Integer) (Variables|Default|GetCurrentFace)) " to " (Utilities|String|ToString(Integer) NewFace)))
    (Variables|Default|SetCurrentFace NewFace)))

(fn GetRotationDot
  (params (Arrow :type Arrow%20Component%20Object%20Reference))
  (return (Math|Vector|DotProduct (Math|Vector|GetForwardVector Arrow) (Math|Vector|MakeVector 0.0 0.0 1.0))))

(fn SpawnGyros
  (bind _returnvalue (Game|SpawnActorfromClass "/Game/Custom/Player/BP_Gyro.BP_Gyro_C" (Math|Transform|MakeTransform "0.000000,0.000000,50000.000000" "0, 0, 0" "1.000000,1.000000,1.000000") "AlwaysSpawn" "MultiplyWithRoot" 0 0))
  (Variables|Misc|SetGyroRef _returnvalue)
  (bind _returnvalue_2 (Game|SpawnActorfromClass "/Game/Custom/Player/BP_GyroPhone.BP_GyroPhone_C" (Math|Transform|MakeTransform "150.000000,0.000000,50000.000000" "0, 0, 0" "1.000000,1.000000,1.000000") "AlwaysSpawn" "MultiplyWithRoot" 0 0))
  (Variables|Misc|SetPhoneGyroRef _returnvalue_2))

(fn SetPlayerBaseLocation
  (bind _radius (Variables|Config|GetRadius))
  (Transformation|SetActorLocation (Math|Vector|MakeVector _radius 0.0 (- _radius (Variables|Config|GetRadiusOffset))) false false))